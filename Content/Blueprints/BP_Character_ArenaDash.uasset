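; Player character for the Arena Dash mode, with a server-launched forward dash on a cooldown.
; Tick counts down the cooldown and copies the start timer and, once the game ends, winner data from the GameState.
; RepNotifies push cooldown, orb score, timer and winner values into the local controller's HUDs, guarded by level-name checks.
; DoBump line-traces ahead to launch another character, but nothing in this Blueprint calls it.
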(event `Server_Dash`
  (`self.LaunchCharacter` (* (`self.GetActorForwardVector`) (`self.DashDistance`)))
  (set `self.CanDash` false)
  (set `self.DashTimeRemaining` (`self.DashCooldown`)))

(event `InputAction|Dash`
  (params (Key :type "Key Structure"))
  (:`Pressed`
    (if (`self.CanDash`)
      (`self.Server_Dash`))))

(event `self.ReceiveTick`
  (params (DeltaSeconds :type "Float (single-precision)"))
  (bind _asbp_game_state_arena_dash (cast `/Game/Blueprints/BP_GameState_ArenaDash` (`GameplayStatics.GetGameState`)))
  (if (`/Game/Blueprints/BP_GameState_ArenaDash.GameEnded` _asbp_game_state_arena_dash)
    (set `self.ScoreWinnerRef` (`/Game/Blueprints/BP_GameState_ArenaDash.ScoreWinner` _asbp_game_state_arena_dash))
    (set `self.nameWinnerRef` (`/Game/Blueprints/BP_GameState_ArenaDash.NameWinner` _asbp_game_state_arena_dash))
    (else
      (set `self.StartingTimerRef` (`/Game/Blueprints/BP_GameState_ArenaDash.StartingTimer` _asbp_game_state_arena_dash))
      (if (<= (`self.StartingTimerRef`) 0.0)
        (bind _returnvalue (`GameplayStatics.GetCurrentLevelName` true))
        (if (== _returnvalue "LevelArenaDash")
          (bind _asbp_controller_arena_dash (cast `/Game/Blueprints/BP_Controller_ArenaDash` (`self.GetLocalViewingPlayerController`)))
          (`Widget.SetVisibility` (`/Game/Blueprints/BP_Widget_ArenaDash.StartingTimer` (`/Game/Blueprints/BP_Controller_ArenaDash.HUDRef` _asbp_controller_arena_dash)) "Collapsed")
          (if (> (`self.DashTimeRemaining`) 0.0) :!label _label
            (set `self.DashTimeRemaining` (- (`self.DashTimeRemaining`) DeltaSeconds))
            (if (<= (`self.DashTimeRemaining`) 0.0)
              (set `self.CanDash` true)
              (set `self.DashTimeRemaining` 0.0))))
        (else
          (goto _label))))))

(fn `DoBump`
  (bind _returnvalue (`self.K2_GetActorLocation`))
  (bind _returnvalue_2 (`self.GetActorForwardVector`))
  (bind _outhit (`KismetSystemLibrary.LineTraceSingle` :`Start` (+ _returnvalue (* _returnvalue_2 (`self.start`))) :`End` (+ _returnvalue (* _returnvalue_2 (`self.maxDistance`))) :`TraceChannel` "TraceTypeQuery3" :`DrawTime` 2.0))
  (bind (_bblockinghit _binitialoverlap _time _distance _location _impactpoint _normal _impactnormal _physmat _hitactor) (`GameplayStatics.BreakHitResult` _outhit))
  (if _bblockinghit
    (bind _asbp_character_arena_dash (cast `/Game/Blueprints/BP_Character_ArenaDash` _hitactor))
    (`self.LaunchCharacter` _asbp_character_arena_dash (* (`self.GetActorForwardVector`) (`self.BumpStrength`)) true true)))

(fn `OnRep_DashTimeRemaining`
  (bind _returnvalue (`GameplayStatics.GetCurrentLevelName` true))
  (if (not (== _returnvalue "LevelHUB"))
    (bind _asbp_controller_arena_dash (cast `/Game/Blueprints/BP_Controller_ArenaDash` (`self.GetLocalViewingPlayerController`)))
    (`ProgressBar.SetPercent` (`/Game/Blueprints/BP_Widget_ArenaDash.ProgressBar_0` (`/Game/Blueprints/BP_Controller_ArenaDash.HUDRef` _asbp_controller_arena_dash)) (- 1.0 (/ (`self.DashTimeRemaining`) (`self.DashCooldown`))))))

(fn `OnRep_nameWinnerRef`
  (bind _returnvalue (`GameplayStatics.GetCurrentLevelName` true))
  (if (== _returnvalue "LevelArenaDash")
    (bind _asbp_controller_arena_dash (cast `/Game/Blueprints/BP_Controller_ArenaDash` (`self.GetLocalViewingPlayerController`)))
    (set `TextBlock.Text` (`self.nameWinnerRef`) (`/Game/Blueprints/BP_EndWidget_ArenaDash.WinnerName` (`/Game/Blueprints/BP_Controller_ArenaDash.HUDGameEndedRef` _asbp_controller_arena_dash)))))

(fn `OnRep_ScoreOrb`
  (bind _returnvalue (`GameplayStatics.GetCurrentLevelName` true))
  (if (not (== _returnvalue "LevelHUB"))
    (bind _asbp_controller_arena_dash (cast `/Game/Blueprints/BP_Controller_ArenaDash` (`self.GetLocalViewingPlayerController`)))
    (set `TextBlock.Text` (`KismetTextLibrary.Conv_IntToText` (`self.ScoreOrb`)) (`/Game/Blueprints/BP_Widget_ArenaDash.TextBlock_1` (`/Game/Blueprints/BP_Controller_ArenaDash.HUDRef` _asbp_controller_arena_dash)))))

(fn `OnRep_ScoreWinnerRef`
  (bind _returnvalue (`GameplayStatics.GetCurrentLevelName` true))
  (if (not (== _returnvalue "LevelHUB"))
    (bind _asbp_controller_arena_dash (cast `/Game/Blueprints/BP_Controller_ArenaDash` (`self.GetLocalViewingPlayerController`)))
    (set `TextBlock.Text` (`KismetTextLibrary.Conv_IntToText` (`self.ScoreWinnerRef`)) (`/Game/Blueprints/BP_EndWidget_ArenaDash.WinnerScore` (`/Game/Blueprints/BP_Controller_ArenaDash.HUDGameEndedRef` _asbp_controller_arena_dash)))))

(fn `OnRep_StartingTimer`)

(fn `OnRep_StartingTimerRef`
  (bind _returnvalue (`GameplayStatics.GetCurrentLevelName` true))
  (if (not (== _returnvalue "LevelHUB"))
    (bind _asbp_controller_arena_dash (cast `/Game/Blueprints/BP_Controller_ArenaDash` (`self.GetLocalViewingPlayerController`)))
    (set `TextBlock.Text` (`KismetTextLibrary.Conv_DoubleToText` (`self.StartingTimerRef`) "HalfToEven") (`/Game/Blueprints/BP_Widget_ArenaDash.StartingTimer` (`/Game/Blueprints/BP_Controller_ArenaDash.HUDRef` _asbp_controller_arena_dash)))))

(fn `UserConstructionScript`
  (`parent.UserConstructionScript`))