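; BP_ToBeReady_ArenaDash is a ready-up plate for Arena Dash that reports to the game mode when it is stepped on or left.
; On the server, begin and end overlap set PlayerOnPlate and PlayerRef, then call PlayerEnteredPlate or PlayerLeftPlate on BP_Gamemode_ArenaDash2.
; Both events use player character 0 instead of the overlapping actor, so any overlap registers as that player.
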(event `self.ReceiveActorBeginOverlap`
  (params (OtherActor :type "Actor Object Reference"))
  (bind _asbp_character_arena_dash (cast `/Game/Blueprints/BP_Character_ArenaDash` (`GameplayStatics.GetPlayerCharacter` 0)))
  (`/Engine/EditorBlueprintResources/ActorMacros.Switch Has Authority`
    (:`Authority`
      (set `self.PlayerOnPlate` true)
      (set `self.PlayerRef` _asbp_character_arena_dash)
      (bind _asbp_gamemode_arena_dash_2 (cast `/Game/Blueprints/BP_Gamemode_ArenaDash2` (`GameplayStatics.GetGameMode`)))
      (`/Game/Blueprints/BP_Gamemode_ArenaDash2.PlayerEnteredPlate` _asbp_gamemode_arena_dash_2))))

(event `self.ReceiveActorEndOverlap`
  (params (OtherActor :type "Actor Object Reference"))
  (cast `/Game/Blueprints/BP_Character_ArenaDash` (`GameplayStatics.GetPlayerCharacter` 0))
  (`/Engine/EditorBlueprintResources/ActorMacros.Switch Has Authority`
    (:`Authority`
      (set `self.PlayerOnPlate` false)
      (set `self.PlayerRef` null)
      (bind _asbp_gamemode_arena_dash_2 (cast `/Game/Blueprints/BP_Gamemode_ArenaDash2` (`GameplayStatics.GetGameMode`)))
      (`/Game/Blueprints/BP_Gamemode_ArenaDash2.PlayerLeftPlate` _asbp_gamemode_arena_dash_2))))

(fn `UserConstructionScript`)