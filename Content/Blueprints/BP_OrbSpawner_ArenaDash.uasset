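; Orb spawner for Arena Dash that scatters BP_Orb_ArenaDash actors across the area of its Box component.
; On BeginPlay, only the authority starts a looping timer that spawns one orb per tick at a random XY inside the box and a fixed world height.
; Each orb receives a reference to the spawner, and the OrbsSpawned counter gates spawning, increasing with every spawn and never decreasing in this Blueprint.
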(event `self.ReceiveBeginPlay`
  (`/Engine/EditorBlueprintResources/ActorMacros.Switch Has Authority`
    (:`Authority`
      (`KismetSystemLibrary.K2_SetTimerDelegate` (delegate `SpawnOrbsEvent`) 2.0 true))))

(event `SpawnOrbsEvent`
  (bind _box (`self.Box`))
  (if (<= (`self.OrbsSpawned`) 10)
    (`|SpawnActorFromClass` "/Game/Blueprints/BP_Orb_ArenaDash.BP_Orb_ArenaDash_C" (`KismetMathLibrary.MakeTransform` (`KismetMathLibrary.MakeVector` (.x (`KismetMathLibrary.RandomPointInBoundingBox` (`SceneComponent.K2_GetComponentLocation` _box) (`BoxComponent.GetScaledBoxExtent` _box))) (.y (`KismetMathLibrary.RandomPointInBoundingBox` (`SceneComponent.K2_GetComponentLocation` _box) (`BoxComponent.GetScaledBoxExtent` _box))) 80.0)) "Undefined" "MultiplyWithRoot" null self null)
    (set `self.OrbsSpawned` (+ (`self.OrbsSpawned`) 1))))

(fn `UserConstructionScript`)