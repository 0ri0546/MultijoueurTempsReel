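; Player controller for Arena Dash that manages local UI, chat, scoreboard and input across the hub and arena levels.
; BeginPlay builds per-level widgets, including an authority-only hub button that server-travels to the arena once two players are on plates.
; Server events relay chat through GameState multicast, trigger character bumps and increment PlayerState score.
; Tick polls GameEnded to swap the HUD for an end screen, creating a new one every frame.
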(event `self.ReceiveBeginPlay`
  (`parent.ReceiveBeginPlay`)
  (if (`self.IsLocalController`)
    (bind _returnvalue (`|CreateWidget` "/Game/Blueprints/BP_TAB_ArenaDash.BP_TAB_ArenaDash_C"))
    (bind _output_get (set `self.ScoreboardWidget` _returnvalue))
    (`UserWidget.AddToViewport` _output_get 0)
    (`Widget.SetVisibility` _returnvalue "Hidden")
    (cast `/Game/Blueprints/BP_GameState_ArenaDash` (`GameplayStatics.GetGameState`))
    (bind _returnvalue_2 (`GameplayStatics.GetCurrentLevelName` true))
    (if (== _returnvalue_2 "LevelHUB")
      (`/Engine/EditorBlueprintResources/ActorMacros.Switch Has Authority`
        (:`Authority`
          (bind _returnvalue_3 (`|CreateWidget` "/Game/Blueprints/BP_WidgetToConfirm_ArenaDash.BP_WidgetToConfirm_ArenaDash_C"))
          (`UserWidget.AddToPlayerScreen` _returnvalue_3 0)
          (add `Button.OnPressed` (`/Game/Blueprints/BP_WidgetToConfirm_ArenaDash.Button_0` _returnvalue_3) (delegate `OnPressed`))))
      (else
        (bind _returnvalue_4 (`GameplayStatics.GetCurrentLevelName` true))
        (if (== _returnvalue_4 "LevelArenaDash")
          (bind _returnvalue_5 (`|CreateWidget` "/Game/Blueprints/BP_Widget_ArenaDash.BP_Widget_ArenaDash_C"))
          (`UserWidget.AddToViewport` _returnvalue_5 0)
          (set `self.HUDRef` _returnvalue_5))))))

(event `OnPressed`
  (bind _asbp_gamemode_arena_dash_2 (cast `/Game/Blueprints/BP_Gamemode_ArenaDash2` (`GameplayStatics.GetGameMode`)))
  (if (>= (`/Game/Blueprints/BP_Gamemode_ArenaDash2.PlayersOnPlate` _asbp_gamemode_arena_dash_2) 2)
    (`KismetSystemLibrary.ExecuteConsoleCommand` "ServerTravel LevelArenaDash?listen" null)))

(event `self.ReceiveTick`
  (params (DeltaSeconds :type "Float (single-precision)"))
  (bind _asbp_game_state_arena_dash (cast `/Game/Blueprints/BP_GameState_ArenaDash` (`GameplayStatics.GetGameState`)))
  (if (`/Game/Blueprints/BP_GameState_ArenaDash.GameEnded` _asbp_game_state_arena_dash)
    (`Widget.RemoveFromParent` (stale `self.ReceiveBeginPlay` _returnvalue_5))
    (bind _returnvalue (`|CreateWidget` "/Game/Blueprints/BP_EndWidget_ArenaDash.BP_EndWidget_ArenaDash_C"))
    (`UserWidget.AddToPlayerScreen` _returnvalue 0)
    (set `self.HUDGameEndedRef` _returnvalue)))

(event `InputAction|OpenChat`
  (params (Key :type "Key Structure"))
  (bind _returnvalue (`self.K2_GetPawn`))
  (:`Pressed`
    (if (`self.IsLocalPlayerController`)
      (if (`self.ChatIsOpen`)
        (`Widget.RemoveFromParent` (stale _returnvalue_2))
        (set `self.ChatIsOpen` false)
        (set `self.bShowMouseCursor` false)
        (`WidgetBlueprintLibrary.SetInputMode_GameOnly` null)
        (`self.EnableInput` _returnvalue null)
        (else
          (bind _returnvalue_2 (`|CreateWidget` "/Game/Blueprints/BP_ChatWidget_ArenaDash.BP_ChatWidget_ArenaDash_C"))
          (set `self.WidgetChatRef` _returnvalue_2)
          (`UserWidget.AddToPlayerScreen` _returnvalue_2 0)
          (set `self.ChatIsOpen` true)
          (set `self.bShowMouseCursor` true)
          (`Widget.SetKeyboardFocus` (`/Game/Blueprints/BP_ChatWidget_ArenaDash.ET_Message` (`self.WidgetChatRef`)))
          (`WidgetBlueprintLibrary.SetInputMode_GameAndUIEx` null (`self.WidgetChatRef`) "DoNotLock" false)
          (`self.DisableInput` _returnvalue null))))))

(event `Server_SendChatMessage`
  (params (Message :type Text))
  (bind _returnvalue (`KismetTextLibrary.Conv_StringToText` (`KismetSystemLibrary.GetDisplayName` self)))
  (bind _asbp_game_state_arena_dash (cast `/Game/Blueprints/BP_GameState_ArenaDash` (`GameplayStatics.GetGameState`)))
  (bind _messageid (`/Game/Blueprints/BP_GameState_ArenaDash.AddChatMessage` _asbp_game_state_arena_dash _returnvalue Message))
  (`/Game/Blueprints/BP_GameState_ArenaDash.Multicast_ReceiveChatMessage` _asbp_game_state_arena_dash _returnvalue Message _messageid))

(event `InputAction|Bump`
  (params (Key :type "Key Structure"))
  (:`Pressed`
    (`self.Server_Bump`)))

(event `Server_Bump`
  (bind _asbp_character_arena_dash (cast `/Game/Blueprints/BP_Character_ArenaDash` (`self.K2_GetPawn`)))
  (`/Game/Blueprints/BP_Character_ArenaDash.DoBump` _asbp_character_arena_dash))

(event `InputAction|OpenListPlayers`
  (params (Key :type "Key Structure"))
  (:`Pressed`
    (`Widget.SetVisibility` (`self.ScoreboardWidget`) "Visible")
    (`/Game/Blueprints/BP_TAB_ArenaDash.RebuildScoreboard` (`self.ScoreboardWidget`)))
  (:`Released`
    (`Widget.SetVisibility` (`self.ScoreboardWidget`) "Hidden")))

(event `Server_AddScore`
  (bind _asbp_player_state_arena_dash (cast `/Game/Blueprints/BP_PlayerState_ArenaDash` (`self.PlayerState`)))
  (set `/Game/Blueprints/BP_PlayerState_ArenaDash.ActualScore` (+ (`/Game/Blueprints/BP_PlayerState_ArenaDash.ActualScore` _asbp_player_state_arena_dash) 1) _asbp_player_state_arena_dash))

(fn `OnRep_Players`)

(fn `UserConstructionScript`
  (`parent.UserConstructionScript`))