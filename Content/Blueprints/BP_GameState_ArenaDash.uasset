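; Game state for Arena Dash that runs the match clock, picks the winner and relays player chat.
; On LevelArenaDash, a server-decremented start countdown sets EnableGame, which Tick turns into the match timer that ends the game.
; Once GameEnded is set, Tick scans players for the highest orb score and records that name.
; Chat reaches controller widgets through a multicast event and a server-appended history replayed by its OnRep.
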(event `self.ReceiveBeginPlay`
  (bind _returnvalue (`GameplayStatics.GetCurrentLevelName` true))
  (if (== _returnvalue "LevelArenaDash")
    ; Start Timer
    (set `self.EnableGame` false)
    (set `self.StartingTimer` (`self.StartingGameDuration`))
    (bind _returnvalue_2 (`KismetSystemLibrary.K2_SetTimerDelegate` (delegate `UpdateSartingTimer`) 1.0 true))
    (set `self.VariableStartingTime` _returnvalue_2)))

(event `self.ReceiveTick`
  (params (DeltaSeconds :type "Float (single-precision)"))
  (if (`self.EnableGame`)
    (set `self.CanOpenMap` true)
    ; Main Timer
    (set `self.TimerGame` (`self.TimerDuration`))
    (bind _returnvalue (`KismetSystemLibrary.K2_SetTimerDelegate` (delegate `UpdateTimer`) 1.0 true))
    (set `self.VariableEventTimer` _returnvalue)
    (set `self.EnableGame` false)
    (elif (`self.GameEnded`)
      ; Set winner score and name
      (for (_ _array_index) (`self.PlayerArray`)
        (bind _asbp_character_arena_dash (cast `/Game/Blueprints/BP_Character_ArenaDash` (`GameplayStatics.GetPlayerCharacter` _array_index)))
        (bind _scoreorb (`/Game/Blueprints/BP_Character_ArenaDash.ScoreOrb` _asbp_character_arena_dash))
        (if (> _scoreorb (`self.ScoreWinner`))
          (bind _output_get (set `self.ScoreWinner` _scoreorb))
          (if (== _output_get _scoreorb)
            (bind _asbp_player_state_arena_dash (cast `/Game/Blueprints/BP_PlayerState_ArenaDash` (`GameplayStatics.GetPlayerState` _array_index)))
            (set `self.NameWinner` (`KismetTextLibrary.Conv_StringToText` (`PlayerState.GetPlayerName` _asbp_player_state_arena_dash)))))))))

(event `UpdateTimer`
  ; Main Timer
  (`/Engine/EditorBlueprintResources/ActorMacros.Switch Has Authority`
    (:`Authority`
      (set `self.TimerGame` (- (`self.TimerGame`) 1.0))
      (if (<= (`self.TimerGame`) 0.0)
        (`KismetSystemLibrary.K2_ClearAndInvalidateTimerHandle` (`self.VariableEventTimer`))
        (set `self.GameEnded` true)))))

(event `UpdateSartingTimer`
  ; Start Timer
  (set `self.CanOpenMap` false)
  (`/Engine/EditorBlueprintResources/ActorMacros.Switch Has Authority`
    (:`Authority`
      (set `self.StartingTimer` (- (`self.StartingTimer`) 1.0))
      (if (<= (`self.StartingTimer`) 0.0)
        (set `self.EnableGame` true)
        (`KismetSystemLibrary.K2_ClearAndInvalidateTimerHandle` (`self.VariableStartingTime`))))))

(event `Multicast_ReceiveChatMessage`
  (params (PlayerName :type Text) (Message :type Text) (MessageID :type Integer))
  ; receive message (chat)
  (for (_ _array_index) (`self.PlayerArray`)
    (bind _asbp_controller_arena_dash (cast `/Game/Blueprints/BP_Controller_ArenaDash` (`GameplayStatics.GetPlayerController` _array_index)))
    (`/Game/Blueprints/BP_ChatWidget_ArenaDash.AddMessage` (`/Game/Blueprints/BP_Controller_ArenaDash.WidgetChatRef` _asbp_controller_arena_dash) Message PlayerName MessageID)))

(fn `AddChatMessage`
  (params (PlayerName :type Text) (Message :type Text))
  (returns (MessageID :type Integer))
  (bind _returnvalue (`KismetMathLibrary.RandomInteger` 999999))
  (`/Engine/EditorBlueprintResources/ActorMacros.Switch Has Authority`
    (:`Authority`
      (`KismetArrayLibrary.Array_Add` (`self.ChatHistoryRef`) (make `/Game/Blueprints/S_ChatMessage_ArenaDash` PlayerName Message _returnvalue))
      (return _returnvalue))))

(fn `GetChatHistoryForPlayer`
  (returns (ChatArray :type "Array of /Game/Blueprints/S_ChatMessage_ArenaDash Structure"))
  (return (`self.ChatHistoryRef`)))

(fn `OnRep_ChatHistoryRef`
  (for (_ _array_index) (`self.PlayerArray`)
    (bind _asbp_controller_arena_dash (cast `/Game/Blueprints/BP_Controller_ArenaDash` (`GameplayStatics.GetPlayerController` _array_index)))
    (for _array_element (`self.ChatHistoryRef`)
      (bind (_playername _message) (break `/Game/Blueprints/S_ChatMessage_ArenaDash` _array_element))
      (`/Game/Blueprints/BP_ChatWidget_ArenaDash.AddMessage` (`/Game/Blueprints/BP_Controller_ArenaDash.WidgetChatRef` _asbp_controller_arena_dash) _message _playername 0))))

(fn `OnRep_PressedStartButton`)

(fn `OnRep_StartingTimer`)

(fn `OnRep_TimerGame`)

(fn `UserConstructionScript`)