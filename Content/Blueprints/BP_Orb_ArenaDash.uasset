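; BP_Orb_ArenaDash is a collectible orb for Arena Dash that scores when a BP_Character_ArenaDash overlaps it.
; On the authority, the overlap first calls ServerAddScore on the character's BP_Controller_ArenaDash, stopping if that controller cast fails.
; Both authority and clients then increment the character's ScoreOrb locally.
; Only the authority decrements the spawner's OrbsSpawned count and destroys the orb.
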(event `self.ReceiveActorBeginOverlap`
  (params (OtherActor :type "Actor Object Reference"))
  (if (`self.HasAuthority`)
    (bind _asbp_character_arena_dash (cast `/Game/Blueprints/BP_Character_ArenaDash` OtherActor))
    (bind _asbp_controller_arena_dash (cast `/Game/Blueprints/BP_Controller_ArenaDash` (`Pawn.GetController` _asbp_character_arena_dash)))
    (`/Game/Blueprints/BP_Controller_ArenaDash.Server_AddScore` _asbp_controller_arena_dash))
  (bind _asbp_character_arena_dash_2 (cast `/Game/Blueprints/BP_Character_ArenaDash` OtherActor))
  (set `/Game/Blueprints/BP_Character_ArenaDash.ScoreOrb` (+ (`/Game/Blueprints/BP_Character_ArenaDash.ScoreOrb` _asbp_character_arena_dash_2) 1) _asbp_character_arena_dash_2)
  (`/Engine/EditorBlueprintResources/ActorMacros.Switch Has Authority`
    (:`Authority`
      (`/Engine/EditorBlueprintResources/StandardMacros.DecrementInt` (`/Game/Blueprints/BP_OrbSpawner_ArenaDash.OrbsSpawned` (`self.SpawnerRef`))
        (:`  `
          (`self.K2_DestroyActor`))))))

(fn `UserConstructionScript`)